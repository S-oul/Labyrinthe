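; Player controller for a first-person labyrinth game with torches, a lever and a trap, announced by a French welcome message on BeginPlay.
; It adds the Move and Actions Enhanced Input mapping contexts, then routes move, look, jump and crouch to the player character and control rotation.
; The action input calls CastLineTrace on the character's ACLineTrace component, with the character found through GetActorOfClass for movement and actions.
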(event `self.ReceiveBeginPlay`
  (bind _returnvalue (pcsubsystem `EnhancedInputLocalPlayerSubsystem` self))
  ;[1 1 1] Set Context
  (`KismetSystemLibrary.PrintText` "Bienvenue dans le Labyrinthe Il y a 3 Torches un levier et un piège faite attention....")
  (`/Engine/EditorBlueprintResources/StandardMacros.IsValid` _returnvalue
    (:`Is Valid`
      (`EnhancedInputSubsystemInterface.AddMappingContext` _returnvalue "/Game/FirstPersonArms/Input/IMC/IMC_Move.IMC_Move" 0 (struct))
      (`EnhancedInputSubsystemInterface.AddMappingContext` _returnvalue "/Game/FirstPersonArms/Input/IMC/IMC_Actions.IMC_Actions" 0 (struct)))))

(event `EnhancedInput|/Game/FirstPersonArms/Input/Inputs/IA_Action`
  (params (ActionValue :type Boolean) (ElapsedSeconds :type "Float (double-precision)") (TriggeredSeconds :type "Float (double-precision)") (InputAction :type "InputAction Object Reference" :default "/Game/FirstPersonArms/Input/Inputs/IA_Action.IA_Action"))
  ;[1 1 1] Torcher?
  (:`Started`
    (bind _returnvalue (`GameplayStatics.GetActorOfClass` "/Game/Le_Labyrinthe/Blueprints/BP_FirstPersonCharacter.BP_FirstPersonCharacter_C"))
    (`/Game/Le_Labyrinthe/Blueprints/Component/AC_LineTrace.Cast Line Trace` (`/Game/Le_Labyrinthe/Blueprints/BP_FirstPersonCharacter.AC_LineTrace` _returnvalue))))

(event `EnhancedInput|/Game/FirstPersonArms/Input/Inputs/Mouvements/IA_Jump`
  (params (ActionValue :type Boolean) (ElapsedSeconds :type "Float (double-precision)") (TriggeredSeconds :type "Float (double-precision)") (InputAction :type "InputAction Object Reference" :default "/Game/FirstPersonArms/Input/Inputs/Mouvements/IA_Jump.IA_Jump"))
  (bind _returnvalue (`GameplayStatics.GetPlayerCharacter` 0))
  ;[1 1 1] Jump Crouch
  (:`Started`
    (`Character.Jump` _returnvalue))
  (:`Completed`
    (`Character.StopJumping` _returnvalue)))

(event `EnhancedInput|/Game/FirstPersonArms/Input/Inputs/Mouvements/IA_Move`
  (params (ActionValue :type "Vector2D Structure") (ElapsedSeconds :type "Float (double-precision)") (TriggeredSeconds :type "Float (double-precision)") (InputAction :type "InputAction Object Reference" :default "/Game/FirstPersonArms/Input/Inputs/Mouvements/IA_Move.IA_Move"))
  (bind (_returnvalue_roll _returnvalue_pitch _returnvalue_yaw) (`KismetMathLibrary.BreakRotator` (`self.GetControlRotation`)))
  ;[1 1 1] Movement
  (:`Triggered`
    (bind _returnvalue (`GameplayStatics.GetActorOfClass` "/Game/Le_Labyrinthe/Blueprints/BP_FirstPersonCharacter.BP_FirstPersonCharacter_C"))
    (`Pawn.AddMovementInput` _returnvalue (`KismetMathLibrary.GetRightVector` (`KismetMathLibrary.MakeRotator` _returnvalue_roll 0.0 _returnvalue_yaw)) ActionValue_X false)
    (`Pawn.AddMovementInput` _returnvalue (`KismetMathLibrary.GetForwardVector` (`KismetMathLibrary.MakeRotator` 0.0 0.0 _returnvalue_yaw)) ActionValue_Y false)))

(event `EnhancedInput|/Game/FirstPersonArms/Input/Inputs/Mouvements/IA_Crouch`
  (params (ActionValue :type Boolean) (ElapsedSeconds :type "Float (double-precision)") (TriggeredSeconds :type "Float (double-precision)") (InputAction :type "InputAction Object Reference" :default "/Game/FirstPersonArms/Input/Inputs/Mouvements/IA_Crouch.IA_Crouch"))
  (bind _returnvalue (`GameplayStatics.GetPlayerCharacter` 0))
  ;[1 1 1] Jump Crouch
  (:`Started`
    (`Character.Crouch` _returnvalue))
  (:`Canceled`
    (`Character.UnCrouch` _returnvalue :!label _label))
  (:`Completed`
    (goto _label)))

(event `EnhancedInput|/Game/FirstPersonArms/Input/Inputs/Mouvements/IA_Look`
  (params (ActionValue :type "Vector2D Structure") (ElapsedSeconds :type "Float (double-precision)") (TriggeredSeconds :type "Float (double-precision)") (InputAction :type "InputAction Object Reference" :default "/Game/FirstPersonArms/Input/Inputs/Mouvements/IA_Look.IA_Look"))
  ;[1 1 1] Camera control
  (:`Triggered`
    (`self.AddYawInput` ActionValue_X)
    (`self.AddPitchInput` ActionValue_Y)))

(fn `UserConstructionScript`)