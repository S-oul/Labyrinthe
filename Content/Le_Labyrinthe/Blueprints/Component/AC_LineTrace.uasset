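; Actor component for the labyrinth's torch-and-lever puzzle, providing the interaction trace that opens the door.
; CastLineTrace runs a short, debug-drawn Visibility trace from the player camera and triggers any torch or lever it hits.
; Torch hits adjust the first-person character's torch count according to the torch's active state.
; After either hit, exactly three counted torches plus an active last-hit lever calls KillDoof on the door.
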(event `Cast Line Trace`
  (bind _returnvalue (`GameplayStatics.GetPlayerCameraManager` 0))
  (bind _player2 (`self.Player2`))
  (bind _player2_2 (`self.Player2`))
  (bind _returnvalue_2 (`SceneComponent.K2_GetComponentLocation` (`Actor.RootComponent` _returnvalue)))
  ;[1 1 1] Set player
  (set `self.player` (`self.GetOwner`))
  (bind _returnvalue_3 (`GameplayStatics.GetActorOfClass` "/Game/Le_Labyrinthe/Blueprints/BP_FirstPersonCharacter.BP_FirstPersonCharacter_C"))
  (set `self.Player2` _returnvalue_3)
  (bind _outhit (`KismetSystemLibrary.LineTraceSingle` :`Start` _returnvalue_2 :`End` (+ _returnvalue_2 (* (`Actor.GetActorForwardVector` _returnvalue) 500)) :`TraceChannel` "TraceTypeQuery1" :`DrawDebugType` "ForDuration"))
  ;[1 1 1] Who are you
  (bind _asbp_torche (cast `/Game/Le_Labyrinthe/Blueprints/BP_Torche` (`.HitActor` (`GameplayStatics.BreakHitResult` _outhit)))
    (:`then`
      ;[1 1 1] Set + Action
      (bind _output_get (set `self.Torche` _asbp_torche))
      (`/Game/Le_Labyrinthe/Blueprints/BP_Torche.Torch Hited` _output_get)
      ;[1 1 1] INcrement or decrement the number of torches
      (if (`/Game/Le_Labyrinthe/Blueprints/BP_Torche.Is active` (`self.Torche`))
        (bind _result (`/Engine/EditorBlueprintResources/StandardMacros.IncrementInt` (`/Game/Le_Labyrinthe/Blueprints/BP_FirstPersonCharacter.nombre de torche` _player2_2))
          (:`  `
            (bind _output_get_2 (set `/Game/Le_Labyrinthe/Blueprints/BP_FirstPersonCharacter.nombre de torche` _result _player2_2))
            (`KismetSystemLibrary.PrintString` (`KismetStringLibrary.Conv_IntToString` _output_get_2))))
        (else
          (bind _result_2 (`/Engine/EditorBlueprintResources/StandardMacros.DecrementInt` (`/Game/Le_Labyrinthe/Blueprints/BP_FirstPersonCharacter.nombre de torche` _player2))
            (:`  `
              (bind _output_get_3 (set `/Game/Le_Labyrinthe/Blueprints/BP_FirstPersonCharacter.nombre de torche` _result_2 _player2))
              (`KismetSystemLibrary.PrintString` (`KismetStringLibrary.Conv_IntToString` _output_get_3))))))
      ;[1 1 1] Verification and Action for door
      (if (== (`/Game/Le_Labyrinthe/Blueprints/BP_FirstPersonCharacter.nombre de torche` (`self.Player2`)) 3) :!label _label
        (if (`/Game/Le_Labyrinthe/Blueprints/BP_lever.Is active` (`self.Lever`))
          (bind _returnvalue_4 (`GameplayStatics.GetActorOfClass` "/Game/Le_Labyrinthe/Blueprints/BP_door.BP_door_C"))
          (`/Game/Le_Labyrinthe/Blueprints/BP_door.Kill  doof` _returnvalue_4))))
    (:`CastFailed`
      (bind _asbp_lever (cast `/Game/Le_Labyrinthe/Blueprints/BP_lever` (`.HitActor` (`GameplayStatics.BreakHitResult` _outhit)))
        (:`then`
          ;[1 1 1] Action and set
          (bind _output_get_4 (set `self.Lever` _asbp_lever))
          (`/Game/Le_Labyrinthe/Blueprints/BP_lever.Hited Lever` _output_get_4)
          (goto _label))
        (:`CastFailed`
          (`KismetSystemLibrary.PrintString` "Nothing in range !"))))))